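; BP_TestEnemy is a test enemy Blueprint that handles the visual and animation response to attack, block, hit and init events.
; OnInit sets the skeletal mesh asset from the EnemySkeletalMesh in LevelData.
; OnAttack, OnBlock and OnHit each play a matching hard-coded Otomatone_2 montage on that mesh, with AnimSpeed as the play rate.
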(event EventOnInit
  (Components|SkeletalMesh|SetSkeletalMeshAsset (Variables|Default|GetSkeletalMesh) (Variables|/Script/MasterRhythmGame.LevelData|GetEnemySkeletalMesh (Variables|Default|GetLevelData))))

(event EventOnAttack
  (Animation|Montage|PlayMontage (Variables|Default|GetSkeletalMesh) "/Game/RythmGame_Art/Animations/AM_Otomatone_2_Attack.AM_Otomatone_2_Attack" (Variables|Default|GetAnimSpeed)))

(event EventOnBlock
  (Animation|Montage|PlayMontage (Variables|Default|GetSkeletalMesh) "/Game/RythmGame_Art/Animations/AM_Otomatone_2_Block.AM_Otomatone_2_Block" (Variables|Default|GetAnimSpeed)))

(event EventOnHit
  (Animation|Montage|PlayMontage (Variables|Default|GetSkeletalMesh) "/Game/RythmGame_Art/Animations/AM_Otomatone_2_Hit.AM_Otomatone_2_Hit" (Variables|Default|GetAnimSpeed)))

(fn ConstructionScript)