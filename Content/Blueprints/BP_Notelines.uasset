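; Actor that draws seven note lines as spline meshes, one for each natural note of a 12-semitone octave.
; The construction script tiles thinned segments along each spline, stacking lines 600 units apart in Z and re-multiplying MeshLength by actor Z scale before each.
; GetSplines and GetSplinesY map a note number modulo 12 to its spline and a Z offset in 150-unit steps, with no case for sharps.
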(event EventBeginPlay)

(event Collision|EventActorBeginOverlap
  (params (OtherActor :type Actor%20Object%20Reference)))

(event EventTick
  (params (DeltaSeconds :type Float%20%28single-precision%29)))

(fn ConstructionScript
  (bind _spline (Variables|Default|GetSpline))
  (bind _spline1 (Variables|Default|GetSpline1))
  (bind _spline1_2 (Variables|Default|GetSpline1))
  (bind _spline_2 (Variables|Default|GetSpline))
  (bind _spline2 (Variables|Default|GetSpline2))
  (bind _spline2_2 (Variables|Default|GetSpline2))
  (bind _spline3 (Variables|Default|GetSpline3))
  (bind _spline3_2 (Variables|Default|GetSpline3))
  (bind _spline4 (Variables|Default|GetSpline4))
  (bind _spline4_2 (Variables|Default|GetSpline4))
  (bind _spline5 (Variables|Default|GetSpline5))
  (bind _spline5_2 (Variables|Default|GetSpline5))
  (bind _spline6 (Variables|Default|GetSpline6))
  (bind _spline6_2 (Variables|Default|GetSpline6))
  (Utilities|FlowControl|Sequence
    (:then_0
      (AddComponent|AddSplineMeshComponent false)
      (Variables|Default|SetMeshLength (* (.z (Transformation|GetActorScale3D)) (Variables|Default|GetMeshLength)))
      (for _index (range 0 (Math|Float|Truncate (- (/ (Spline|GetSplineLength (Variables|Default|GetSpline)) (Variables|Default|GetMeshLength)) 1.0)))
        (bind _returnvalue (AddComponent|AddSplineMeshComponent false))
        (SplineMesh|SetStartandEnd _returnvalue (Spline|GetLocationatDistanceAlongSpline _spline (* _index (Variables|Default|GetMeshLength)) "Local") (Math|Vector|ClampVectorSize (Spline|GetTangentatDistanceAlongSpline _spline (* _index (Variables|Default|GetMeshLength)) "Local") 0.0 (Variables|Default|GetMeshLength)) (Spline|GetLocationatDistanceAlongSpline _spline_2 (* (+ _index 1) (Variables|Default|GetMeshLength)) "Local") (Math|Vector|ClampVectorSize (Spline|GetTangentatDistanceAlongSpline _spline_2 (* (+ _index 1) (Variables|Default|GetMeshLength)) "Local") 0.0 (Variables|Default|GetMeshLength)) true :!class /Script/Engine.SplineMeshComponent)
        (Transformation|SetRelativeScale3D _returnvalue "1.000000,0.250000,0.250000")))
    (:then_1
      (AddComponent|AddSplineMeshComponent false)
      (Variables|Default|SetMeshLength (* (.z (Transformation|GetActorScale3D)) (Variables|Default|GetMeshLength)))
      (for _index_2 (range 0 (Math|Float|Truncate (- (/ (Spline|GetSplineLength (Variables|Default|GetSpline1)) (Variables|Default|GetMeshLength)) 1.0)))
        (bind _returnvalue_2 (AddComponent|AddSplineMeshComponent false))
        (SplineMesh|SetStartandEnd _returnvalue_2 (Math|Vector|MakeVector (.x (Spline|GetLocationatDistanceAlongSpline _spline1_2 (* _index_2 (Variables|Default|GetMeshLength)) "Local")) (.y (Spline|GetLocationatDistanceAlongSpline _spline1_2 (* _index_2 (Variables|Default|GetMeshLength)) "Local")) (+ (.z (Spline|GetLocationatDistanceAlongSpline _spline1_2 (* _index_2 (Variables|Default|GetMeshLength)) "Local")) 6e+02)) (Math|Vector|ClampVectorSize (Spline|GetTangentatDistanceAlongSpline _spline1_2 (* _index_2 (Variables|Default|GetMeshLength)) "Local") 0.0 (Variables|Default|GetMeshLength)) (Math|Vector|MakeVector (.x (Spline|GetLocationatDistanceAlongSpline _spline1 (* (+ _index_2 1) (Variables|Default|GetMeshLength)) "Local")) (.y (Spline|GetLocationatDistanceAlongSpline _spline1 (* (+ _index_2 1) (Variables|Default|GetMeshLength)) "Local")) (+ (.z (Spline|GetLocationatDistanceAlongSpline _spline1 (* (+ _index_2 1) (Variables|Default|GetMeshLength)) "Local")) 6e+02)) (Math|Vector|ClampVectorSize (Spline|GetTangentatDistanceAlongSpline _spline1 (* (+ _index_2 1) (Variables|Default|GetMeshLength)) "Local") 0.0 (Variables|Default|GetMeshLength)) true :!class /Script/Engine.SplineMeshComponent)
        (Transformation|SetRelativeScale3D _returnvalue_2 "1.000000,0.250000,0.250000")))
    (:then_2
      (AddComponent|AddSplineMeshComponent false)
      (Variables|Default|SetMeshLength (* (.z (Transformation|GetActorScale3D)) (Variables|Default|GetMeshLength)))
      (for _index_3 (range 0 (Math|Float|Truncate (- (/ (Spline|GetSplineLength (Variables|Default|GetSpline2)) (Variables|Default|GetMeshLength)) 1.0)))
        (bind _returnvalue_3 (AddComponent|AddSplineMeshComponent false))
        (SplineMesh|SetStartandEnd _returnvalue_3 (Math|Vector|MakeVector (.x (Spline|GetLocationatDistanceAlongSpline _spline2 (* _index_3 (Variables|Default|GetMeshLength)) "Local")) (.y (Spline|GetLocationatDistanceAlongSpline _spline2 (* _index_3 (Variables|Default|GetMeshLength)) "Local")) (+ (.z (Spline|GetLocationatDistanceAlongSpline _spline2 (* _index_3 (Variables|Default|GetMeshLength)) "Local")) 1.2e+03)) (Math|Vector|ClampVectorSize (Spline|GetTangentatDistanceAlongSpline _spline2 (* _index_3 (Variables|Default|GetMeshLength)) "Local") 0.0 (Variables|Default|GetMeshLength)) (Math|Vector|MakeVector (.x (Spline|GetLocationatDistanceAlongSpline _spline2_2 (* (+ _index_3 1) (Variables|Default|GetMeshLength)) "Local")) (.y (Spline|GetLocationatDistanceAlongSpline _spline2_2 (* (+ _index_3 1) (Variables|Default|GetMeshLength)) "Local")) (+ (.z (Spline|GetLocationatDistanceAlongSpline _spline2_2 (* (+ _index_3 1) (Variables|Default|GetMeshLength)) "Local")) 1.2e+03)) (Math|Vector|ClampVectorSize (Spline|GetTangentatDistanceAlongSpline _spline2_2 (* (+ _index_3 1) (Variables|Default|GetMeshLength)) "Local") 0.0 (Variables|Default|GetMeshLength)) true :!class /Script/Engine.SplineMeshComponent)
        (Transformation|SetRelativeScale3D _returnvalue_3 "1.000000,0.250000,0.250000")))
    (:then_3
      (AddComponent|AddSplineMeshComponent false)
      (Variables|Default|SetMeshLength (* (.z (Transformation|GetActorScale3D)) (Variables|Default|GetMeshLength)))
      (for _index_4 (range 0 (Math|Float|Truncate (- (/ (Spline|GetSplineLength (Variables|Default|GetSpline3)) (Variables|Default|GetMeshLength)) 1.0)))
        (bind _returnvalue_4 (AddComponent|AddSplineMeshComponent false))
        (SplineMesh|SetStartandEnd _returnvalue_4 (Math|Vector|MakeVector (.x (Spline|GetLocationatDistanceAlongSpline _spline3 (* _index_4 (Variables|Default|GetMeshLength)) "Local")) (.y (Spline|GetLocationatDistanceAlongSpline _spline3 (* _index_4 (Variables|Default|GetMeshLength)) "Local")) (+ (.z (Spline|GetLocationatDistanceAlongSpline _spline3 (* _index_4 (Variables|Default|GetMeshLength)) "Local")) 1.8e+03)) (Math|Vector|ClampVectorSize (Spline|GetTangentatDistanceAlongSpline _spline3 (* _index_4 (Variables|Default|GetMeshLength)) "Local") 0.0 (Variables|Default|GetMeshLength)) (Math|Vector|MakeVector (.x (Spline|GetLocationatDistanceAlongSpline _spline3_2 (* (+ _index_4 1) (Variables|Default|GetMeshLength)) "Local")) (.y (Spline|GetLocationatDistanceAlongSpline _spline3_2 (* (+ _index_4 1) (Variables|Default|GetMeshLength)) "Local")) (+ (.z (Spline|GetLocationatDistanceAlongSpline _spline3_2 (* (+ _index_4 1) (Variables|Default|GetMeshLength)) "Local")) 1.8e+03)) (Math|Vector|ClampVectorSize (Spline|GetTangentatDistanceAlongSpline _spline3_2 (* (+ _index_4 1) (Variables|Default|GetMeshLength)) "Local") 0.0 (Variables|Default|GetMeshLength)) true :!class /Script/Engine.SplineMeshComponent)
        (Transformation|SetRelativeScale3D _returnvalue_4 "1.000000,0.250000,0.250000")))
    (:then_4
      (AddComponent|AddSplineMeshComponent false)
      (Variables|Default|SetMeshLength (* (.z (Transformation|GetActorScale3D)) (Variables|Default|GetMeshLength)))
      (for _index_5 (range 0 (Math|Float|Truncate (- (/ (Spline|GetSplineLength (Variables|Default|GetSpline4)) (Variables|Default|GetMeshLength)) 1.0)))
        (bind _returnvalue_5 (AddComponent|AddSplineMeshComponent false))
        (SplineMesh|SetStartandEnd _returnvalue_5 (Math|Vector|MakeVector (.x (Spline|GetLocationatDistanceAlongSpline _spline4 (* _index_5 (Variables|Default|GetMeshLength)) "Local")) (.y (Spline|GetLocationatDistanceAlongSpline _spline4 (* _index_5 (Variables|Default|GetMeshLength)) "Local")) (+ (.z (Spline|GetLocationatDistanceAlongSpline _spline4 (* _index_5 (Variables|Default|GetMeshLength)) "Local")) 2.4e+03)) (Math|Vector|ClampVectorSize (Spline|GetTangentatDistanceAlongSpline _spline4 (* _index_5 (Variables|Default|GetMeshLength)) "Local") 0.0 (Variables|Default|GetMeshLength)) (Math|Vector|MakeVector (.x (Spline|GetLocationatDistanceAlongSpline _spline4_2 (* (+ _index_5 1) (Variables|Default|GetMeshLength)) "Local")) (.y (Spline|GetLocationatDistanceAlongSpline _spline4_2 (* (+ _index_5 1) (Variables|Default|GetMeshLength)) "Local")) (+ (.z (Spline|GetLocationatDistanceAlongSpline _spline4_2 (* (+ _index_5 1) (Variables|Default|GetMeshLength)) "Local")) 2.4e+03)) (Math|Vector|ClampVectorSize (Spline|GetTangentatDistanceAlongSpline _spline4_2 (* (+ _index_5 1) (Variables|Default|GetMeshLength)) "Local") 0.0 (Variables|Default|GetMeshLength)) true :!class /Script/Engine.SplineMeshComponent)
        (Transformation|SetRelativeScale3D _returnvalue_5 "1.000000,0.250000,0.250000")))
    (:then_5
      (AddComponent|AddSplineMeshComponent false)
      (Variables|Default|SetMeshLength (* (.z (Transformation|GetActorScale3D)) (Variables|Default|GetMeshLength)))
      (for _index_6 (range 0 (Math|Float|Truncate (- (/ (Spline|GetSplineLength (Variables|Default|GetSpline5)) (Variables|Default|GetMeshLength)) 1.0)))
        (bind _returnvalue_6 (AddComponent|AddSplineMeshComponent false))
        (SplineMesh|SetStartandEnd _returnvalue_6 (Math|Vector|MakeVector (.x (Spline|GetLocationatDistanceAlongSpline _spline5 (* _index_6 (Variables|Default|GetMeshLength)) "Local")) (.y (Spline|GetLocationatDistanceAlongSpline _spline5 (* _index_6 (Variables|Default|GetMeshLength)) "Local")) (+ (.z (Spline|GetLocationatDistanceAlongSpline _spline5 (* _index_6 (Variables|Default|GetMeshLength)) "Local")) 3e+03)) (Math|Vector|ClampVectorSize (Spline|GetTangentatDistanceAlongSpline _spline5 (* _index_6 (Variables|Default|GetMeshLength)) "Local") 0.0 (Variables|Default|GetMeshLength)) (Math|Vector|MakeVector (.x (Spline|GetLocationatDistanceAlongSpline _spline5_2 (* (+ _index_6 1) (Variables|Default|GetMeshLength)) "Local")) (.y (Spline|GetLocationatDistanceAlongSpline _spline5_2 (* (+ _index_6 1) (Variables|Default|GetMeshLength)) "Local")) (+ (.z (Spline|GetLocationatDistanceAlongSpline _spline5_2 (* (+ _index_6 1) (Variables|Default|GetMeshLength)) "Local")) 3e+03)) (Math|Vector|ClampVectorSize (Spline|GetTangentatDistanceAlongSpline _spline5_2 (* (+ _index_6 1) (Variables|Default|GetMeshLength)) "Local") 0.0 (Variables|Default|GetMeshLength)) true :!class /Script/Engine.SplineMeshComponent)
        (Transformation|SetRelativeScale3D _returnvalue_6 "1.000000,0.250000,0.250000")))
    (:then_6
      (AddComponent|AddSplineMeshComponent false)
      (Variables|Default|SetMeshLength (* (.z (Transformation|GetActorScale3D)) (Variables|Default|GetMeshLength)))
      (for _index_7 (range 0 (Math|Float|Truncate (- (/ (Spline|GetSplineLength (Variables|Default|GetSpline6)) (Variables|Default|GetMeshLength)) 1.0)))
        (bind _returnvalue_7 (AddComponent|AddSplineMeshComponent false))
        (SplineMesh|SetStartandEnd _returnvalue_7 (Math|Vector|MakeVector (.x (Spline|GetLocationatDistanceAlongSpline _spline6_2 (* _index_7 (Variables|Default|GetMeshLength)) "Local")) (.y (Spline|GetLocationatDistanceAlongSpline _spline6_2 (* _index_7 (Variables|Default|GetMeshLength)) "Local")) (+ (.z (Spline|GetLocationatDistanceAlongSpline _spline6_2 (* _index_7 (Variables|Default|GetMeshLength)) "Local")) 3.6e+03)) (Math|Vector|ClampVectorSize (Spline|GetTangentatDistanceAlongSpline _spline6_2 (* _index_7 (Variables|Default|GetMeshLength)) "Local") 0.0 (Variables|Default|GetMeshLength)) (Math|Vector|MakeVector (.x (Spline|GetLocationatDistanceAlongSpline _spline6 (* (+ _index_7 1) (Variables|Default|GetMeshLength)) "Local")) (.y (Spline|GetLocationatDistanceAlongSpline _spline6 (* (+ _index_7 1) (Variables|Default|GetMeshLength)) "Local")) (+ (.z (Spline|GetLocationatDistanceAlongSpline _spline6 (* (+ _index_7 1) (Variables|Default|GetMeshLength)) "Local")) 3.6e+03)) (Math|Vector|ClampVectorSize (Spline|GetTangentatDistanceAlongSpline _spline6 (* (+ _index_7 1) (Variables|Default|GetMeshLength)) "Local") 0.0 (Variables|Default|GetMeshLength)) true :!class /Script/Engine.SplineMeshComponent)
        (Transformation|SetRelativeScale3D _returnvalue_7 "1.000000,0.250000,0.250000")))))

(fn GetSplines
  (params (Int :type Integer))
  (switch int (Math|Integer|%(Integer) Int 12)
    (:0
      (return (Variables|Default|GetSpline)))
    (:2
      (return (Variables|Default|GetSpline1)))
    (:4
      (return (Variables|Default|GetSpline2)))
    (:5
      (return (Variables|Default|GetSpline3)))
    (:7
      (return (Variables|Default|GetSpline4)))
    (:9
      (return (Variables|Default|GetSpline5)))
    (:11
      (return (Variables|Default|GetSpline6)))))

(fn GetSplinesY
  (params (Int :type Integer))
  (switch int (Math|Integer|%(Integer) Int 12)
    (:0
      (return "0, 0, 0"))
    (:2
      (return "0.000000,0.000000,150.000000"))
    (:4
      (return "0.000000,0.000000,300.000000"))
    (:5
      (return "0.000000,0.000000,450.000000"))
    (:7
      (return "0.000000,0.000000,600.000000"))
    (:9
      (return "0.000000,0.000000,750.000000"))
    (:11
      (return "0.000000,0.000000,900.000000"))))