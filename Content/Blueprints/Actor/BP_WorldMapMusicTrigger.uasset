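; World map music trigger volume that switches the music as the player's world map character enters or leaves its collider.
; Entering fires the start trigger parameter and leaving fires the stop trigger parameter on the Music component of the world map player controller.
; BeginPlay also fires the start trigger if the player pawn already overlaps the collider.
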(event OnComponentBeginOverlap(Collider)
  (params (OverlappedComponent :type Primitive%20Component%20Object%20Reference) (OtherActor :type Actor%20Object%20Reference) (OtherComp :type Primitive%20Component%20Object%20Reference) (OtherBodyIndex :type Integer) (bFromSweep :type Boolean) (SweepResult :type Hit%20Result%20Structure%20%28by%20ref%29))
  (Class|KismetSystemLibrary|IsObjectOfSoftClass OtherActor "/Game/Blueprints/Character/BP_WorldMapCharacter.BP_WorldMapCharacter_C"
    (:True
      (bind _asbp_world_map_controller (Utilities|Casting|CastToBP_WorldMapController (Game|GetPlayerController 0)))
      (Class|AudioParameterControllerInterface|SetTriggerParameter (Variables|/Game/Blueprints/Controller/BP_WorldMapController.BP_WorldMapController_C|GetMusic _asbp_world_map_controller) (Variables|Default|GetStartTriggerName)))))

(event OnComponentEndOverlap(Collider)
  (params (OverlappedComponent :type Primitive%20Component%20Object%20Reference) (OtherActor :type Actor%20Object%20Reference) (OtherComp :type Primitive%20Component%20Object%20Reference) (OtherBodyIndex :type Integer))
  (Class|KismetSystemLibrary|IsObjectOfSoftClass OtherActor "/Game/Blueprints/Character/BP_WorldMapCharacter.BP_WorldMapCharacter_C"
    (:True
      (bind _asbp_world_map_controller (Utilities|Casting|CastToBP_WorldMapController (Game|GetPlayerController 0)))
      (Class|AudioParameterControllerInterface|SetTriggerParameter (Variables|/Game/Blueprints/Controller/BP_WorldMapController.BP_WorldMapController_C|GetMusic _asbp_world_map_controller) (Variables|Default|GetStopTriggerName)))))

(event EventBeginPlay
  (bind _asbp_world_map_character (Utilities|Casting|CastToBP_WorldMapCharacter (Game|Player|GetPlayerPawn 0)))
  (if (Collision|IsOverlappingActor (Variables|Default|GetCollider) _asbp_world_map_character :!class /Script/Engine.PrimitiveComponent)
    (bind _asbp_world_map_controller (Utilities|Casting|CastToBP_WorldMapController (Game|GetPlayerController 0)))
    (Class|AudioParameterControllerInterface|SetTriggerParameter (Variables|/Game/Blueprints/Controller/BP_WorldMapController.BP_WorldMapController_C|GetMusic _asbp_world_map_controller) (Variables|Default|GetStartTriggerName))))

(fn ConstructionScript)