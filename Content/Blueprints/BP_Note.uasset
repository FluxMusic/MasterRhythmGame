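; BP_Note is a rhythm combat projectile that travels along a spline between the player and an attack enemy.
; A Timeline drives its position, playing forward or in reverse, and damages the enemy or player depending on the end reached, then destroys itself.
; Any cone overlap destroys the note early, incrementing the player's Defended count if it hit the player.
; SetBarLength scales the Timeline play rate from BPM, based on four-beat bars.
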(event OnComponentBeginOverlap(Cone)
  (params (OverlappedComponent :type Primitive%20Component%20Object%20Reference) (OtherActor :type Actor%20Object%20Reference) (OtherComp :type Primitive%20Component%20Object%20Reference) (OtherBodyIndex :type Integer) (bFromSweep :type Boolean) (SweepResult :type Hit%20Result%20Structure%20%28by%20ref%29))
  (bind _asbp_player (Utilities|Casting|CastToBP_Player OtherActor)
    (:then
      (Math|Integer|IncrementInt (Variables|/Game/Blueprints/BP_Player.BP_Player_C|GetDefended _asbp_player)
        (:%20%20
          (Actor|DestroyActor))))
    (:CastFailed
      (Actor|DestroyActor))))

(event Custom|MoveRIght
  (bind _alpha (Timeline|Timeline ReverseFromEnd)
    (:Update
      (Transformation|SetWorldLocation (Variables|Default|GetDefaultSceneRoot) (Spline|GetLocationatTime (Variables|Default|GetSplineRef) _alpha "World" false) false false))
    (:Finished
      (if (<= _alpha 0.0)
        (bind _asbp_player (Utilities|Casting|CastToBP_Player (Game|GetPlayerCharacter 0)))
        (Default|ApplyDamage _asbp_player 5)
        (Actor|DestroyActor :!label _label)
        (elif (>= _alpha 1.0)
          (bind _returnvalue (Actor|GetActorOfClass "/Game/Blueprints/AI/AttackAI/BP_AttackEnemy.BP_AttackEnemy_C"))
          (Default|ApplyDamage _returnvalue 5)
          (goto _label))))))

(event Custom|MoveLeft
  (bind _alpha (Timeline|Timeline PlayFromStart)
    (:Update
      (Transformation|SetWorldLocation (Variables|Default|GetDefaultSceneRoot) (Spline|GetLocationatTime (Variables|Default|GetSplineRef) _alpha "World" false) false false))
    (:Finished
      (if (<= _alpha 0.0)
        (bind _asbp_player (Utilities|Casting|CastToBP_Player (Game|GetPlayerCharacter 0)))
        (Default|ApplyDamage _asbp_player 5)
        (Actor|DestroyActor :!label _label)
        (elif (>= _alpha 1.0)
          (bind _returnvalue (Actor|GetActorOfClass "/Game/Blueprints/AI/AttackAI/BP_AttackEnemy.BP_AttackEnemy_C"))
          (Default|ApplyDamage _returnvalue 5)
          (goto _label))))))

(fn ConstructionScript)

(fn SetBarLength
  (params (BPM :type Float%20%28double-precision%29))
  (Components|Timeline|SetPlayRate (Variables|Default|GetTimeline) (/ 1.0 (/ 2.4e+02 BPM))))