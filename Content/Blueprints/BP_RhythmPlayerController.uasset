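; Player controller for a rhythm game that lets a MIDI keyboard move BP_Player and drive menus.
; BeginPlay opens a hardcoded MIDI device; note-ons route by ControllerState to gameplay, pause menu or settings menu handling.
; In-game notes teleport the player between preset Points or pause; in the pause menu they focus, highlight and trigger buttons.
; Enhanced Input offers up, down and pause; other MIDI events only print debug text.
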(event Custom|OnMidiNoteOn
  (params (MIDIDeviceController :type MIDI%20Device%20Input%20Controller%20Object%20Reference) (Timestamp :type Integer) (Channel :type Integer) (Note :type Integer) (Velocity :type Integer))
  ;[0.15 0.15 0.15 0.5] Used for Keys
  (Development|PrintText (Utilities|Text|FormatText "Channel: {Channel}, Note: {Note}, Velocity: {Velocity}" Channel Note Velocity) true true "(R=0.000000,G=0.660000,B=1.000000,A=1.000000)" 1e+01)
  (CallFunction|PlayerMovement Note))

(event Custom|OnPitchwheelBend
  (params (MIDIDeviceController :type MIDI%20Device%20Input%20Controller%20Object%20Reference) (Timestamp :type Integer) (Channel :type Integer) (Pitch :type Integer))
  ;[0.15 0.15 0.15 0.5] Used for Pitch Bend
  (Development|PrintText (Utilities|Text|FormatText "Channel: {Channel}, Pitch: {Pitch}" Channel Pitch) true true "(R=0.000000,G=0.660000,B=1.000000,A=1.000000)" 1e+01))

(event Custom|OnMidiControlChange
  (params (MIDIDeviceController :type MIDI%20Device%20Input%20Controller%20Object%20Reference) (Timestamp :type Integer) (Channel :type Integer) (Type :type Integer) (Value :type Integer))
  ;[0.15 0.15 0.15 0.5] Used for Mod Wheel
  (Development|PrintText (Utilities|Text|FormatText "Channel: {Channel}, Type: {Type}, Value: {Value}" Channel Type Value) true true "(R=0.000000,G=0.660000,B=1.000000,A=1.000000)" 1e+01))

(event Custom|OnMidiAftertouch
  (params (MIDIDeviceController :type MIDI%20Device%20Input%20Controller%20Object%20Reference) (Timestamp :type Integer) (Channel :type Integer) (Note :type Integer) (Amount :type Integer))
  ;[0.15 0.15 0.15 0.5] Could be used for Aftertouch
  (Development|PrintText (Utilities|Text|FormatText "Channel: {Channel}, Note: {Note}, Amount: {Amount}" Channel Note Amount) true true "(R=0.400323,G=1.000000,B=0.000000,A=1.000000)" 1e+01))

(event Input|EnhancedActionEvents|EnhancedInputActionIA_Up
  (params (ActionValue :type Boolean) (ElapsedSeconds :type Float%20%28double-precision%29) (TriggeredSeconds :type Float%20%28double-precision%29) (InputAction :type Input%20Action%20Object%20Reference :default "/Game/Input/InputActions/IA_Up.IA_Up"))
  (:Started
    (bind _asbp_player (Utilities|Casting|CastToBP_Player (Game|GetPlayerCharacter 0)))
    (Transformation|SetWorldLocation (Variables|/Script/Engine.Character|GetCapsuleComponent (stale Input|EnhancedActionEvents|EnhancedInputActionIA_Down _asbp_player)) (Utilities|Array|Get(acopy) (Variables|/Game/Blueprints/BP_Player.BP_Player_C|GetPoints _asbp_player)) false false)))

(event Input|EnhancedActionEvents|EnhancedInputActionIA_Down
  (params (ActionValue :type Boolean) (ElapsedSeconds :type Float%20%28double-precision%29) (TriggeredSeconds :type Float%20%28double-precision%29) (InputAction :type Input%20Action%20Object%20Reference :default "/Game/Input/InputActions/IA_Down.IA_Down"))
  (:Started
    (bind _asbp_player (Utilities|Casting|CastToBP_Player (Game|GetPlayerCharacter 0)))
    (Transformation|SetWorldLocation (Variables|/Script/Engine.Character|GetCapsuleComponent _asbp_player) (Utilities|Array|Get(acopy) (Variables|/Game/Blueprints/BP_Player.BP_Player_C|GetPoints _asbp_player) 1) false false)))

(event Input|EnhancedActionEvents|EnhancedInputActionIA_Pause
  (params (ActionValue :type Boolean) (ElapsedSeconds :type Float%20%28double-precision%29) (TriggeredSeconds :type Float%20%28double-precision%29) (InputAction :type Input%20Action%20Object%20Reference :default "/Game/Input/InputActions/IA_Pause.IA_Pause"))
  (:Started
    (CallFunction|PauseGame)))

(event EventBeginPlay
  (bind _midicontroller (Variables|Default|GetMidiController))
  ;[0.15 0.15 0.15 0.5] Debug
  (CallFunction|DisplayMidiDeviceIDs)
  (CallFunction|DisplayDefaultMidiDeviceID)
  (CallFunction|CreateMidiController)
  (EventDispatchers|BindEventtoOnMIDINoteon _midicontroller (delegate Custom|OnMidiNoteOn))
  (EventDispatchers|BindEventtoOnMIDIPitchBend _midicontroller (delegate Custom|OnPitchwheelBend))
  (EventDispatchers|BindEventtoOnMIDIControlChange _midicontroller (delegate Custom|OnMidiControlChange))
  (EventDispatchers|BindEventtoOnMIDIAftertouch _midicontroller (delegate Custom|OnMidiAftertouch))
  (Input|AddMappingContext (PlayerController|LocalPlayerSubsystems|GetEnhancedInputLocalPlayerSubsystem (Game|GetPlayerController 0)) "/Game/Input/IMC_Default.IMC_Default" 0 "(bIgnoreAllPressedKeysUntilRelease=True,bForceImmediately=False,bNotifyUserSettings=False)"))

(fn ConstructionScript)

(fn DisplayMidiDeviceIDs
  (bind _outmididevices (Class|MIDIDeviceManager|FindMIDIDevices))
  (for _array_element _outmididevices
    (Development|PrintText (Utilities|Text|FormatText "ID: {ID}, Name: {Name}" (.DeviceID (Utilities|Struct|BreakFoundMIDIDevice _array_element)) (.DeviceName (Utilities|Struct|BreakFoundMIDIDevice _array_element))) true true "(R=0.000000,G=0.660000,B=1.000000,A=1.000000)" 1e+01)))

(fn DisplayDefaultMidiDeviceID
  (bind _deviceid (Class|MIDIDeviceManager|GetDefaultMIDIInputDeviceID))
  (Development|PrintText (Utilities|Text|FormatText "Default Device ID: {ID}" _deviceid)))

(fn CreateMidiController
  (bind _returnvalue (Class|MIDIDeviceManager|CreateMIDIDeviceInputController 1 1024))
  (Variables|Default|SetMidiController _returnvalue))

(fn PlayerMovement
  (params (i_Note :type Integer))
  (switch Utilities|FlowControl|Switch|SwitchonE_ControllerState (Variables|Default|GetControllerState)
    (:NewEnumerator1
      (CallFunction|PauseMenu i_Note))
    (:NewEnumerator2
      (bind _asbp_menu_controller (Utilities|Casting|CastToBP_MenuController (Game|GetPlayerController 0)))
      (Default|SettingMenuControl _asbp_menu_controller i_Note))
    (:NewEnumerator9
      (switch string (Utilities|String|ToString(Integer) i_Note)
        (:41
          (bind _asbp_player (Utilities|Casting|CastToBP_Player (Game|GetPlayerCharacter 0)))
          (Transformation|SetWorldLocation (Variables|/Script/Engine.Character|GetCapsuleComponent _asbp_player) (Utilities|Array|Get(acopy) (Variables|/Game/Blueprints/BP_Player.BP_Player_C|GetPoints _asbp_player)) false false))
        (:43
          (bind _asbp_player_2 (Utilities|Casting|CastToBP_Player (Game|GetPlayerCharacter 0)))
          (Transformation|SetWorldLocation (Variables|/Script/Engine.Character|GetCapsuleComponent _asbp_player_2) (Utilities|Array|Get(acopy) (Variables|/Game/Blueprints/BP_Player.BP_Player_C|GetPoints _asbp_player_2) 1) false false))
        (:45
          (bind _asbp_player_3 (Utilities|Casting|CastToBP_Player (Game|GetPlayerCharacter 0)))
          (Transformation|SetWorldLocation (Variables|/Script/Engine.Character|GetCapsuleComponent _asbp_player_3) (Utilities|Array|Get(acopy) (Variables|/Game/Blueprints/BP_Player.BP_Player_C|GetPoints _asbp_player_3) 2) false false))
        (:47
          (bind _asbp_player_4 (Utilities|Casting|CastToBP_Player (Game|GetPlayerCharacter 0)))
          (Transformation|SetWorldLocation (Variables|/Script/Engine.Character|GetCapsuleComponent _asbp_player_4) (Utilities|Array|Get(acopy) (Variables|/Game/Blueprints/BP_Player.BP_Player_C|GetPoints _asbp_player_4) 3) false false))
        (:48
          (bind _asbp_player_5 (Utilities|Casting|CastToBP_Player (Game|GetPlayerCharacter 0)))
          (Transformation|SetWorldLocation (Variables|/Script/Engine.Character|GetCapsuleComponent _asbp_player_5) (Utilities|Array|Get(acopy) (Variables|/Game/Blueprints/BP_Player.BP_Player_C|GetPoints _asbp_player_5) 4) false false))
        (:50
          (bind _asbp_player_6 (Utilities|Casting|CastToBP_Player (Game|GetPlayerCharacter 0)))
          (Transformation|SetWorldLocation (Variables|/Script/Engine.Character|GetCapsuleComponent _asbp_player_6) (Utilities|Array|Get(acopy) (Variables|/Game/Blueprints/BP_Player.BP_Player_C|GetPoints _asbp_player_6) 5) false false))
        (:52
          (bind _asbp_player_7 (Utilities|Casting|CastToBP_Player (Game|GetPlayerCharacter 0)))
          (Transformation|SetWorldLocation (Variables|/Script/Engine.Character|GetCapsuleComponent _asbp_player_7) (Utilities|Array|Get(acopy) (Variables|/Game/Blueprints/BP_Player.BP_Player_C|GetPoints _asbp_player_7) 6) false false))
        (:70
          (CallFunction|PauseGame))))))

(fn PauseGame
  (bind _returnvalue (Game|GetPlayerController 0))
  (bind _returnvalue_2 (HUD|GetHUD _returnvalue))
  (bind _asbp_hud (Utilities|Casting|CastToBP_HUD _returnvalue_2))
  (Widget|SetVisibility (Variables|/Game/Blueprints/UI/BP_HUD.BP_HUD_C|GetMainUIRef _asbp_hud) "Hidden")
  (Game|SetGamePaused true)
  (bind _asbp_hud_2 (Utilities|Casting|CastToBP_HUD _returnvalue_2))
  (Widget|SetVisibility (Variables|/Game/Blueprints/UI/BP_HUD.BP_HUD_C|GetPauseRef _asbp_hud_2) "Visible")
  (Variables|/Script/Engine.PlayerController|SetbShowMouseCursor (Game|GetPlayerController 0) true)
  (Variables|Default|SetControllerState "NewEnumerator1")
  (Widget|SetKeyboardFocus (Variables|/Game/Blueprints/UI/WBP_PauseMenu.WBP_PauseMenu_C|GetResume_Button (Variables|/Game/Blueprints/UI/BP_HUD.BP_HUD_C|GetPauseRef _asbp_hud_2)))
  (Class|Button|SetBackgroundColor (Variables|/Game/Blueprints/UI/WBP_PauseMenu.WBP_PauseMenu_C|GetResume_Button (Variables|/Game/Blueprints/UI/BP_HUD.BP_HUD_C|GetPauseRef _asbp_hud_2)) "(R=0.207717,G=1.000000,B=0.328281,A=1.000000)"))

(fn PauseMenu
  (params (InInt :type Integer))
  (bind _returnvalue (Game|GetPlayerController 0))
  (bind _returnvalue_2 (HUD|GetHUD _returnvalue))
  (switch string (Utilities|String|ToString(Integer) InInt)
    (:41
      (bind _asbp_hud (Utilities|Casting|CastToBP_HUD _returnvalue_2))
      (Widget|SetKeyboardFocus (Variables|/Game/Blueprints/UI/WBP_PauseMenu.WBP_PauseMenu_C|GetResume_Button (Variables|/Game/Blueprints/UI/BP_HUD.BP_HUD_C|GetPauseRef _asbp_hud)))
      (bind _asbp_hud_2 (Utilities|Casting|CastToBP_HUD (HUD|GetHUD (Game|GetPlayerController 0))))
      (Class|Button|SetBackgroundColor (Variables|/Game/Blueprints/UI/WBP_PauseMenu.WBP_PauseMenu_C|GetSave_Button (Variables|/Game/Blueprints/UI/BP_HUD.BP_HUD_C|GetPauseRef _asbp_hud_2)) "(R=1.000000,G=1.000000,B=1.000000,A=1.000000)")
      (Class|Button|SetBackgroundColor (Variables|/Game/Blueprints/UI/WBP_PauseMenu.WBP_PauseMenu_C|GetResume_Button (Variables|/Game/Blueprints/UI/BP_HUD.BP_HUD_C|GetPauseRef _asbp_hud_2)) "(R=0.207717,G=1.000000,B=0.328281,A=1.000000)"))
    (:43
      (bind _asbp_hud_3 (Utilities|Casting|CastToBP_HUD _returnvalue_2))
      (Widget|SetKeyboardFocus (Variables|/Game/Blueprints/UI/WBP_PauseMenu.WBP_PauseMenu_C|GetSave_Button (Variables|/Game/Blueprints/UI/BP_HUD.BP_HUD_C|GetPauseRef _asbp_hud_3)))
      (bind _asbp_hud_4 (Utilities|Casting|CastToBP_HUD (HUD|GetHUD (Game|GetPlayerController 0))))
      (Class|Button|SetBackgroundColor (Variables|/Game/Blueprints/UI/WBP_PauseMenu.WBP_PauseMenu_C|GetLoad_Button (Variables|/Game/Blueprints/UI/BP_HUD.BP_HUD_C|GetPauseRef _asbp_hud_4)) "(R=1.000000,G=1.000000,B=1.000000,A=1.000000)")
      (Class|Button|SetBackgroundColor (Variables|/Game/Blueprints/UI/WBP_PauseMenu.WBP_PauseMenu_C|GetSave_Button (Variables|/Game/Blueprints/UI/BP_HUD.BP_HUD_C|GetPauseRef _asbp_hud_4)) "(R=0.207717,G=1.000000,B=0.328281,A=1.000000)"))
    (:45
      (bind _asbp_hud_5 (Utilities|Casting|CastToBP_HUD _returnvalue_2))
      (Widget|SetKeyboardFocus (Variables|/Game/Blueprints/UI/WBP_PauseMenu.WBP_PauseMenu_C|GetLoad_Button (Variables|/Game/Blueprints/UI/BP_HUD.BP_HUD_C|GetPauseRef _asbp_hud_5)))
      (bind _asbp_hud_6 (Utilities|Casting|CastToBP_HUD (HUD|GetHUD (Game|GetPlayerController 0))))
      (Class|Button|SetBackgroundColor (Variables|/Game/Blueprints/UI/WBP_PauseMenu.WBP_PauseMenu_C|GetSettings_Button (Variables|/Game/Blueprints/UI/BP_HUD.BP_HUD_C|GetPauseRef _asbp_hud_6)) "(R=1.000000,G=1.000000,B=1.000000,A=1.000000)")
      (Class|Button|SetBackgroundColor (Variables|/Game/Blueprints/UI/WBP_PauseMenu.WBP_PauseMenu_C|GetLoad_Button (Variables|/Game/Blueprints/UI/BP_HUD.BP_HUD_C|GetPauseRef _asbp_hud_6)) "(R=0.207717,G=1.000000,B=0.328281,A=1.000000)"))
    (:47
      (bind _asbp_hud_7 (Utilities|Casting|CastToBP_HUD _returnvalue_2))
      (Widget|SetKeyboardFocus (Variables|/Game/Blueprints/UI/WBP_PauseMenu.WBP_PauseMenu_C|GetSettings_Button (Variables|/Game/Blueprints/UI/BP_HUD.BP_HUD_C|GetPauseRef _asbp_hud_7)))
      (bind _asbp_hud_8 (Utilities|Casting|CastToBP_HUD (HUD|GetHUD (Game|GetPlayerController 0))))
      (Class|Button|SetBackgroundColor (Variables|/Game/Blueprints/UI/WBP_PauseMenu.WBP_PauseMenu_C|GetMainMenu_Button (Variables|/Game/Blueprints/UI/BP_HUD.BP_HUD_C|GetPauseRef _asbp_hud_8)) "(R=1.000000,G=1.000000,B=1.000000,A=1.000000)")
      (Class|Button|SetBackgroundColor (Variables|/Game/Blueprints/UI/WBP_PauseMenu.WBP_PauseMenu_C|GetSettings_Button (Variables|/Game/Blueprints/UI/BP_HUD.BP_HUD_C|GetPauseRef _asbp_hud_8)) "(R=0.207717,G=1.000000,B=0.328281,A=1.000000)"))
    (:48
      (bind _asbp_hud_9 (Utilities|Casting|CastToBP_HUD _returnvalue_2))
      (Widget|SetKeyboardFocus (Variables|/Game/Blueprints/UI/WBP_PauseMenu.WBP_PauseMenu_C|GetMainMenu_Button (Variables|/Game/Blueprints/UI/BP_HUD.BP_HUD_C|GetPauseRef _asbp_hud_9)))
      (bind _asbp_hud_10 (Utilities|Casting|CastToBP_HUD (HUD|GetHUD (Game|GetPlayerController 0))))
      (Class|Button|SetBackgroundColor (Variables|/Game/Blueprints/UI/WBP_PauseMenu.WBP_PauseMenu_C|GetQuit_Button (Variables|/Game/Blueprints/UI/BP_HUD.BP_HUD_C|GetPauseRef _asbp_hud_10)) "(R=1.000000,G=1.000000,B=1.000000,A=1.000000)")
      (Class|Button|SetBackgroundColor (Variables|/Game/Blueprints/UI/WBP_PauseMenu.WBP_PauseMenu_C|GetMainMenu_Button (Variables|/Game/Blueprints/UI/BP_HUD.BP_HUD_C|GetPauseRef _asbp_hud_10)) "(R=0.207717,G=1.000000,B=0.328281,A=1.000000)"))
    (:50
      (bind _asbp_hud_11 (Utilities|Casting|CastToBP_HUD _returnvalue_2))
      (Widget|SetKeyboardFocus (Variables|/Game/Blueprints/UI/WBP_PauseMenu.WBP_PauseMenu_C|GetQuit_Button (Variables|/Game/Blueprints/UI/BP_HUD.BP_HUD_C|GetPauseRef _asbp_hud_11)))
      (bind _asbp_hud_12 (Utilities|Casting|CastToBP_HUD (HUD|GetHUD (Game|GetPlayerController 0))))
      (Class|Button|SetBackgroundColor (Variables|/Game/Blueprints/UI/WBP_PauseMenu.WBP_PauseMenu_C|GetResume_Button (Variables|/Game/Blueprints/UI/BP_HUD.BP_HUD_C|GetPauseRef _asbp_hud_12)) "(R=1.000000,G=1.000000,B=1.000000,A=1.000000)")
      (Class|Button|SetBackgroundColor (Variables|/Game/Blueprints/UI/WBP_PauseMenu.WBP_PauseMenu_C|GetQuit_Button (Variables|/Game/Blueprints/UI/BP_HUD.BP_HUD_C|GetPauseRef _asbp_hud_12)) "(R=0.207717,G=1.000000,B=0.328281,A=1.000000)"))
    (:72
      (bind _asbp_hud_13 (Utilities|Casting|CastToBP_HUD _returnvalue_2))
      (if (Class|Widget|HasKeyboardFocus (Variables|/Game/Blueprints/UI/WBP_PauseMenu.WBP_PauseMenu_C|GetResume_Button (Variables|/Game/Blueprints/UI/BP_HUD.BP_HUD_C|GetPauseRef _asbp_hud_13)))
        (Default|Resume (Variables|/Game/Blueprints/UI/BP_HUD.BP_HUD_C|GetPauseRef _asbp_hud_13))
        (elif (Class|Widget|HasKeyboardFocus (Variables|/Game/Blueprints/UI/WBP_PauseMenu.WBP_PauseMenu_C|GetSave_Button (Variables|/Game/Blueprints/UI/BP_HUD.BP_HUD_C|GetPauseRef _asbp_hud_13)))
          (Default|SaveGame (Variables|/Game/Blueprints/UI/BP_HUD.BP_HUD_C|GetPauseRef _asbp_hud_13))
          (elif (Class|Widget|HasKeyboardFocus (Variables|/Game/Blueprints/UI/WBP_PauseMenu.WBP_PauseMenu_C|GetLoad_Button (Variables|/Game/Blueprints/UI/BP_HUD.BP_HUD_C|GetPauseRef _asbp_hud_13)))
            (Default|LoadGame (Variables|/Game/Blueprints/UI/BP_HUD.BP_HUD_C|GetPauseRef _asbp_hud_13))
            (elif (Class|Widget|HasKeyboardFocus (Variables|/Game/Blueprints/UI/WBP_PauseMenu.WBP_PauseMenu_C|GetSettings_Button (Variables|/Game/Blueprints/UI/BP_HUD.BP_HUD_C|GetPauseRef _asbp_hud_13)))
              (Default|Settings (Variables|/Game/Blueprints/UI/BP_HUD.BP_HUD_C|GetPauseRef _asbp_hud_13))
              (elif (Class|Widget|HasKeyboardFocus (Variables|/Game/Blueprints/UI/WBP_PauseMenu.WBP_PauseMenu_C|GetMainMenu_Button (Variables|/Game/Blueprints/UI/BP_HUD.BP_HUD_C|GetPauseRef _asbp_hud_13)))
                (Default|MainMenu (Variables|/Game/Blueprints/UI/BP_HUD.BP_HUD_C|GetPauseRef _asbp_hud_13))
                (elif (Class|Widget|HasKeyboardFocus (Variables|/Game/Blueprints/UI/WBP_PauseMenu.WBP_PauseMenu_C|GetQuit_Button (Variables|/Game/Blueprints/UI/BP_HUD.BP_HUD_C|GetPauseRef _asbp_hud_13)))
                  (Default|Quit (Variables|/Game/Blueprints/UI/BP_HUD.BP_HUD_C|GetPauseRef _asbp_hud_13)))))))))))