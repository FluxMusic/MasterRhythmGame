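; BP_AttackEnemy is an enemy actor that fires BP_Note projectiles, takes damage and tracks its own health.
; Attack spawns a note at its Scene offset, and notes overlapping its Box get their X velocity altered.
; ApplyDamage updates Health through CalcHealth and pushes it to the HUD's enemy health display.
; At zero or below, the actor destroys itself and swaps the main UI for the death screen.
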(event OnComponentBeginOverlap(Box)
  (params (OverlappedComponent :type Primitive%20Component%20Object%20Reference) (OtherActor :type Actor%20Object%20Reference) (OtherComp :type Primitive%20Component%20Object%20Reference) (OtherBodyIndex :type Integer) (bFromSweep :type Boolean) (SweepResult :type Hit%20Result%20Structure%20%28by%20ref%29))
  (bind _asbp_note (Utilities|Casting|CastToBP_Note OtherActor))
  (bind _result (Math|Float|NegateFloat (.x (Variables|/Script/Engine.MovementComponent|GetVelocity (Variables|/Game/Blueprints/BP_Note.BP_Note_C|GetProjectileMovement _asbp_note))))
    (:%20%20
      (Variables|/Script/Engine.MovementComponent|SetVelocity (Variables|/Game/Blueprints/BP_Note.BP_Note_C|GetProjectileMovement _asbp_note) (Math|Vector|MakeVector _result (.y (Variables|/Script/Engine.MovementComponent|GetVelocity (Variables|/Game/Blueprints/BP_Note.BP_Note_C|GetProjectileMovement _asbp_note))) (.z (Variables|/Script/Engine.MovementComponent|GetVelocity (Variables|/Game/Blueprints/BP_Note.BP_Note_C|GetProjectileMovement _asbp_note))))))))

(event Custom|Attack
  (Game|SpawnActorfromClass "/Game/Blueprints/BP_Note.BP_Note_C" (Math|Transform|MakeTransform (+ (Transformation|GetActorLocation) (Variables|/Script/Engine.SceneComponent|GetRelativeLocation (Variables|Default|GetScene))) (Transformation|GetActorRotation) "1.000000,1.000000,1.000000") "Undefined" "MultiplyWithRoot" 0 0))

(event EventApplyDamage
  (params (DamageAmount :type Integer))
  (bind _output_get (CallFunction|CalcHealth DamageAmount))
  (CallFunction|UI)
  (Math|Integer|CompareInt _output_get
    (:==
      _)
    (:<
      _))
  (Development|PrintString "Damage")
  (Actor|DestroyActor)
  (bind _asbp_hud (Utilities|Casting|CastToBP_HUD (HUD|GetHUD (Game|GetPlayerController 0))))
  (Widget|SetVisibility (Variables|/Game/Blueprints/UI/BP_HUD.BP_HUD_C|GetMainUIRef _asbp_hud) "Hidden")
  (Widget|SetVisibility (Variables|/Game/Blueprints/UI/BP_HUD.BP_HUD_C|GetDeathRef _asbp_hud) "Visible"))

(fn ConstructionScript)

(fn CalcHealth
  (params (Value :type Integer%20%28by%20ref%29))
  (bind _result (Utilities|NegateInt Value)
    (:%20%20
      (bind _output_get (Variables|Default|SetHealth (+ _result (Variables|Default|GetHealth))))
      (return _output_get))))

(fn UI
  (bind _asbp_hud (Utilities|Casting|CastToBP_HUD (HUD|GetHUD (Game|GetPlayerController 0))))
  (Default|SetHealthEnemy (Variables|/Game/Blueprints/UI/BP_HUD.BP_HUD_C|GetMainUIRef _asbp_hud) (Variables|Default|GetHealth))
  (return))