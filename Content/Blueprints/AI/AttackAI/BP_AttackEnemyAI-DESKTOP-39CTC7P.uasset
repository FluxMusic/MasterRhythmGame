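; AI controller that drives BP_AttackEnemy attacks in time with music from a MetaSound.
; After a short startup delay it plays the audio, triggers the melody and music, and watches the MetaSound's MidiNote output.
; Each note is reduced modulo 12; the seven natural notes teleport the controlled enemy to one of seven fixed heights and call Attack.
; It also caches a BP_Notelines reference, unused in this graph.
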(event Custom|MidiNote
  (params (OutputName :type Name) (Output :type Meta%20Sound%20Output%20Structure%20%28by%20ref%29))
  (bind (_success _returnvalue) (Class|MetasoundOutputBlueprintAccess|GetInt32 Output))
  (Development|PrintString (Utilities|String|ToString(Integer) _returnvalue) _success)
  (bind _output_get (Variables|Default|SetMidiInt _returnvalue))
  (bind _asbp_attack_enemy (Utilities|Casting|CastToBP_AttackEnemy (Pawn|GetControlledPawn self)))
  (switch int (Math|Integer|%(Integer) _output_get 12)
    (:0
      (Transformation|SetWorldLocation (Variables|/Script/Engine.Actor|GetRootComponent _asbp_attack_enemy) "100.000000,-2930.000000,100.000000" false false)
      (Default|Attack _asbp_attack_enemy))
    (:2
      (Transformation|SetWorldLocation (Variables|/Script/Engine.Actor|GetRootComponent _asbp_attack_enemy) "100.000000,-2930.000000,250.000000" false false)
      (Default|Attack _asbp_attack_enemy))
    (:4
      (Transformation|SetWorldLocation (Variables|/Script/Engine.Actor|GetRootComponent _asbp_attack_enemy) "100.000000,-2930.000000,400.000000" false false)
      (Default|Attack _asbp_attack_enemy))
    (:5
      (Transformation|SetWorldLocation (Variables|/Script/Engine.Actor|GetRootComponent _asbp_attack_enemy) "100.000000,-2930.000000,550.000000" false false)
      (Default|Attack _asbp_attack_enemy))
    (:7
      (Transformation|SetWorldLocation (Variables|/Script/Engine.Actor|GetRootComponent _asbp_attack_enemy) "100.000000,-2930.000000,700.000000" false false)
      (Default|Attack _asbp_attack_enemy))
    (:9
      (Transformation|SetWorldLocation (Variables|/Script/Engine.Actor|GetRootComponent _asbp_attack_enemy) "100.000000,-2930.000000,850.000000" false false)
      (Default|Attack _asbp_attack_enemy))
    (:11
      (Transformation|SetWorldLocation (Variables|/Script/Engine.Actor|GetRootComponent _asbp_attack_enemy) "100.000000,-2930.000000,1000.000000" false false)
      (Default|Attack _asbp_attack_enemy))))

(event EventBeginPlay
  (bind _audio (Variables|Default|GetAudio))
  (Utilities|FlowControl|Delay 2.5)
  (Audio|Components|Audio|Play _audio 0.0)
  (Class|AudioParameterControllerInterface|SetTriggerParameter _audio "PlayMelody")
  (Class|AudioParameterControllerInterface|SetTriggerParameter _audio "PlayMusic")
  (MetaSoundOutput|WatchOutput (WorldSubsystems|GetMetaSoundOutputSubsystem) _audio "MidiNote" (delegate Custom|MidiNote) "None" "None" :!class /Script/MetasoundEngine.MetaSoundOutputSubsystem)
  (bind _returnvalue (Actor|GetActorOfClass "/Game/Blueprints/BP_Notelines.BP_Notelines_C"))
  (Variables|Default|SetNotelinesRef _returnvalue))

(fn ConstructionScript)