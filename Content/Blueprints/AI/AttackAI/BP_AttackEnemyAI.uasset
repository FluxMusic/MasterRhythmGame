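; AI controller that moves its BP_AttackEnemy pawn between note lines and makes it attack in time with MetaSound music.
; A Quartz clock at the set BPM starts the audio on a bar, triggers melody and music on successive bars after a delay, then stops.
; Each watched MidiNote output selects a BP_Notelines spline, repositions the pawn at its end and calls Attack with the BPM.
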(event EventBeginPlay
  (CallFunction|CreateandStartQuartzClock (Variables|Default|GetBPM))
  (Audio|Components|Audio|PlayQuantized (Variables|Default|GetAudio) (Variables|Default|GetClockHandle) (Utilities|Struct|MakeQuartzQuantizationBoundary "Bar" 1.0 "BarRelative") 0)
  (MetaSoundOutput|WatchOutput (WorldSubsystems|GetMetaSoundOutputSubsystem) (Variables|Default|GetAudio) "MidiNote" (EventDispatchers|CreateEvent :!event OnMidiNoteChange) "None" "None" :!class /Script/MetasoundEngine.MetaSoundOutputSubsystem)
  (bind _returnvalue (Actor|GetActorOfClass "/Game/Blueprints/BP_Notelines.BP_Notelines_C"))
  (Variables|Default|SetNotelinesRef _returnvalue))

(fn ConstructionScript)

(fn CreateandStartQuartzClock
  (params (BPM :type Float%20%28double-precision%29))
  (bind _returnvalue (Class|QuartzSubsystem|CreateNewClock :self (WorldSubsystems|GetQuartzSubsystem) :ClockName "AI"))
  (bind _output_get (Variables|Default|SetClockHandle _returnvalue))
  (bind _clockhandle (Class|QuartzClockHandle|SetBeatsPerMinute :self _output_get :BeatsPerMinute BPM))
  (bind _clockhandle_2 (Class|QuartzClockHandle|SubscribetoQuantizationEvent _clockhandle "Bar" (EventDispatchers|CreateEvent :!event OnQuartzClockBar)))
  (bind _clockhandle_3 (Class|QuartzClockHandle|SubscribetoQuantizationEvent _clockhandle_2 "Beat" (EventDispatchers|CreateEvent :!event OnQuartzClockBeat)))
  (Class|QuartzClockHandle|StartClock _clockhandle_3))

(fn OnQuartzClockBar
  (params (ClockName :type Name) (QuantizationType :type EQuartzCommandQuantization%20Enum :default "Bar") (NumBars :type Integer) (Beat :type Integer) (BeatFraction :type Float%20%28single-precision%29))
  (if (and (== NumBars (+ (Variables|Default|GetNumBarsDelay) 1)) (Audio|Components|Audio|IsPlaying (Variables|Default|GetAudio)))
    (Class|AudioParameterControllerInterface|SetTriggerParameter (Variables|Default|GetAudio) "PlayMelody"))
  (if (and (>= NumBars (+ (Variables|Default|GetNumBarsDelay) 2)) (Audio|Components|Audio|IsPlaying (Variables|Default|GetAudio)))
    (Class|AudioParameterControllerInterface|SetTriggerParameter (Variables|Default|GetAudio) "PlayMusic")
    (Class|QuartzClockHandle|StopClock (Variables|Default|GetClockHandle) true)))

(fn OnQuartzClockBeat
  (params (ClockName :type Name) (QuantizationType :type EQuartzCommandQuantization%20Enum :default "Bar") (NumBars :type Integer) (Beat :type Integer) (BeatFraction :type Float%20%28single-precision%29))
  (Development|PrintString (Utilities|String|ToString(Integer) Beat) true true "(R=0.000000,G=1.000000,B=0.066989,A=1.000000)"))

(fn OnMidiNoteChange
  (params (OutputName :type Name) (Output :type Meta%20Sound%20Output%20Structure%20%28by%20ref%29))
  (bind _notelinesref (Variables|Default|GetNotelinesRef))
  (bind (_success _returnvalue) (Class|MetasoundOutputBlueprintAccess|GetInt32 Output))
  (Development|PrintString (Utilities|String|ToString(Integer) _returnvalue) _success)
  (bind _output_get (Variables|Default|SetMidiInt _returnvalue))
  (bind _asbp_attack_enemy (Utilities|Casting|CastToBP_AttackEnemy (Pawn|GetControlledPawn self)))
  (bind _spline (Default|GetSplines _notelinesref _output_get))
  (bind _output_get_2 (Variables|/Game/Blueprints/AI/AttackAI/BP_AttackEnemy.BP_AttackEnemy_C|SetSplineRef _asbp_attack_enemy _spline))
  (bind _newparam (Default|GetSplinesY _notelinesref (Variables|Default|GetMidiInt)))
  (Transformation|SetActorLocation _asbp_attack_enemy (+ _newparam (+ (Transformation|GetActorLocation _notelinesref) (.position (Spline|GetSplinePointAt _output_get_2 (Spline|GetNumberOfSplinePoints _output_get_2) "World")))) false false)
  (Default|Attack _asbp_attack_enemy (Variables|Default|GetBPM)))