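; BP_AttackEnemy is an enemy actor that attacks by spawning notes and tracks its own health.
; Attack spawns a BP_Note at an offset from the actor, clears its spline reference and starts it moving left.
; ApplyDamage updates health and pushes it to the main HUD widget.
; At zero or below, it destroys the actor, swaps the main UI for the death screen and changes the player controller's state.
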(event Custom|Attack
  (bind _returnvalue (Game|SpawnActorfromClass "/Game/Blueprints/BP_Note.BP_Note_C" (Math|Transform|MakeTransform (+ (Transformation|GetActorLocation) (Variables|/Script/Engine.SceneComponent|GetRelativeLocation (Variables|Default|GetScene))) (Transformation|GetActorRotation) "1.000000,1.000000,1.000000") "Undefined" "MultiplyWithRoot" 0 0))
  (Actor|GetActorOfClass "/Game/Blueprints/BP_Notelines.BP_Notelines_C")
  (Variables|/Game/Blueprints/BP_Note.BP_Note_C|SetSplineRef _returnvalue 0)
  (Default|MoveLeft _returnvalue))

(event EventApplyDamage
  (params (DamageAmount :type Integer))
  (bind _output_get (CallFunction|CalcHealth DamageAmount))
  (CallFunction|UI)
  (Math|Integer|CompareInt _output_get
    (:==
      _)
    (:<
      _))
  (Development|PrintString "Damage")
  (Actor|DestroyActor)
  (bind _asbp_hud (Utilities|Casting|CastToBP_HUD (HUD|GetHUD (Game|GetPlayerController 0))))
  (Widget|SetVisibility (Variables|/Game/Blueprints/UI/BP_HUD.BP_HUD_C|GetMainUIRef _asbp_hud) "Hidden")
  (Widget|SetVisibility (Variables|/Game/Blueprints/UI/BP_HUD.BP_HUD_C|GetDeathRef _asbp_hud) "Visible")
  (bind _asbp_player_controller (Utilities|Casting|CastToBP_PlayerController (Game|GetPlayerController 0)))
  (Variables|/Game/Blueprints/BP_PlayerController.BP_PlayerController_C|SetControllerState _asbp_player_controller "NewEnumerator10"))

(fn ConstructionScript)

(fn CalcHealth
  (params (Value :type Integer%20%28by%20ref%29))
  (bind _result (Utilities|NegateInt Value)
    (:%20%20
      (bind _output_get (Variables|Default|SetHealth (+ _result (Variables|Default|GetHealth))))
      (return _output_get))))

(fn UI
  (bind _asbp_hud (Utilities|Casting|CastToBP_HUD (HUD|GetHUD (Game|GetPlayerController 0))))
  (Default|SetHealthEnemy (Variables|/Game/Blueprints/UI/BP_HUD.BP_HUD_C|GetMainUIRef _asbp_hud) (Variables|Default|GetHealth))
  (return))