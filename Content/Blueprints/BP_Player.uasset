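; BP_Player is the player Blueprint, which tracks health, interacts with BP_Note projectiles and views the game through a designated CameraActor.
; ApplyDamage updates Health through CalcHealth, pushes it to the BP_HUD main UI, and destroys the player when the result is zero or below.
; Box overlaps with a BP_Note modify the X component of its projectile velocity, leaving Y and Z unchanged.
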(event OnComponentBeginOverlap(Box)
  (params (OverlappedComponent :type Primitive%20Component%20Object%20Reference) (OtherActor :type Actor%20Object%20Reference) (OtherComp :type Primitive%20Component%20Object%20Reference) (OtherBodyIndex :type Integer) (bFromSweep :type Boolean) (SweepResult :type Hit%20Result%20Structure%20%28by%20ref%29))
  (bind _asbp_note (Utilities|Casting|CastToBP_Note OtherActor))
  (bind _result (Math|Float|NegateFloat (.x (Variables|/Script/Engine.MovementComponent|GetVelocity (Variables|/Game/Blueprints/BP_Note.BP_Note_C|GetProjectileMovement _asbp_note))))
    (:%20%20
      (Variables|/Script/Engine.MovementComponent|SetVelocity (Variables|/Game/Blueprints/BP_Note.BP_Note_C|GetProjectileMovement _asbp_note) (Math|Vector|MakeVector _result (.y (Variables|/Script/Engine.MovementComponent|GetVelocity (Variables|/Game/Blueprints/BP_Note.BP_Note_C|GetProjectileMovement _asbp_note))) (.z (Variables|/Script/Engine.MovementComponent|GetVelocity (Variables|/Game/Blueprints/BP_Note.BP_Note_C|GetProjectileMovement _asbp_note))))))))

(event EventApplyDamage
  (params (DamageAmount :type Integer))
  (bind _output_get (CallFunction|CalcHealth DamageAmount))
  (CallFunction|UI)
  (Math|Integer|CompareInt _output_get
    (:==
      _)
    (:<
      _))
  (Development|PrintString "Damage")
  (Actor|DestroyActor))

(event EventBeginPlay
  (Game|Player|SetViewTargetwithBlend (Game|GetPlayerController 0) (Utilities|ResolveSoftReference (Variables|Default|GetCameraActor)) 0.0 "VTBlend_Linear" 0.0 false))

(fn ConstructionScript)

(fn CalcHealth
  (params (Value :type Integer%20%28by%20ref%29))
  (bind _result (Utilities|NegateInt Value)
    (:%20%20
      (bind _output_get (Variables|Default|SetHealth (+ _result (Variables|Default|GetHealth))))
      (return _output_get))))

(fn UI
  (bind _asbp_hud (Utilities|Casting|CastToBP_HUD (HUD|GetHUD (Game|GetPlayerController 0))))
  (Default|SetHealth (Variables|/Game/Blueprints/UI/BP_HUD.BP_HUD_C|GetMainUIRef _asbp_hud) (Variables|Default|GetHealth))
  (return))