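; Game character Blueprint that gives an Otomatone character its combat animation and audio feedback for attack, block and hit events.
; Each event plays its montage at AnimSpeed.
; Blocking also triggers the Hit audio component, pitched by passing the last played note, offset by 60, as a MidiNote parameter.
; Hits pick a MetaSound by current level name, while older block-sound logic remains disconnected.
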(event EventOnBlock
  (bind _hit_ (Variables|Default|GetHit%20))
  (Animation|PlayAnimMontage "/Game/RythmGame_Art/Animations/AM_Otomatone_2_Block.AM_Otomatone_2_Block" (Variables|Default|GetAnimSpeed) "None")
  (Audio|Components|Audio|Play _hit_ 0.0)
  (Effects|Components|ParticleSystem|SetIntParameter _hit_ "MidiNote" (- (Class|GameCharacter|GetLastPlayedNote) 60))
  (Class|AudioParameterControllerInterface|SetTriggerParameter _hit_ "Play"))

(event EventOnHit
  (Animation|PlayAnimMontage "/Game/RythmGame_Art/Animations/AM_Otomatone_2_Hit.AM_Otomatone_2_Hit" (Variables|Default|GetAnimSpeed) "None")
  (bind _returnvalue (Game|GetCurrentLevelName true))
  (switch string _returnvalue
    (:MAP_Swamp
      (Audio|PlaySound2D "/Game/Audio/SFX/SFX/META_Combat_Hit_Swamp.META_Combat_Hit_Swamp" 1.0 1.0 0.0 0 0))
    (:MAP_Cyberpunk
      (Audio|PlaySound2D "/Game/Audio/SFX/SFX/META_Combat_Hit_Cyberpunk.META_Combat_Hit_Cyberpunk" 1.0 1.0 0.0 0 0))
    (:MAP_Galaxy
      (Audio|PlaySound2D "/Game/Audio/SFX/SFX/META_Combat_Hit_Galaxy.META_Combat_Hit_Galaxy" 1.0 1.0 0.0 0 0))
    (:MAP_Vulcano
      (Audio|PlaySound2D "/Game/Audio/SFX/SFX/META_Combat_Hit_Vulcano.META_Combat_Hit_Vulcano" 1.0 1.0 0.0 0 0))
    (:TestMap
      (Audio|PlaySound2D "/Game/Audio/SFX/SFX/META_Combat_Hit_Swamp.META_Combat_Hit_Swamp" 1.0 1.0 0.0 0 0))
    (:MAP_Ice
      (Audio|PlaySound2D "/Game/Audio/SFX/SFX/META_Combat_Hit_Ice.META_Combat_Hit_Ice" 1.0 1.0 0.0 0 0))
    (:MAP_Steampunk
      (Audio|PlaySound2D "/Game/Audio/SFX/SFX/META_Combat_Hit_Steampunk.META_Combat_Hit_Steampunk" 1.0 1.0 0.0 0 0))))

(event EventOnAttack
  (Animation|PlayAnimMontage "/Game/RythmGame_Art/Animations/AM_Otomatone_2_Attack.AM_Otomatone_2_Attack" (Variables|Default|GetAnimSpeed) "None"))

(fn ConstructionScript)