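; BP_SplineTest is a test actor that tiles spline mesh segments along its spline at construction time.
; The construction script multiplies MeshLength by the actor's Z scale, then adds one segment per whole length that fits along the spline.
; Each segment takes local-space positions and tangents at its ends, with tangents clamped to MeshLength.
; An extra unconfigured spline mesh precedes the loop, and the event graph is inactive.
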(event EventBeginPlay)

(event Collision|EventActorBeginOverlap
  (params (OtherActor :type Actor%20Object%20Reference)))

(event EventTick
  (params (DeltaSeconds :type Float%20%28single-precision%29)))

(fn ConstructionScript
  (bind _spline (Variables|Default|GetSpline))
  (bind _spline_2 (Variables|Default|GetSpline))
  (AddComponent|AddSplineMeshComponent false)
  (Variables|Default|SetMeshLength (* (.z (Transformation|GetActorScale3D)) (Variables|Default|GetMeshLength)))
  (for _index (range 0 (Math|Float|Truncate (- (/ (Spline|GetSplineLength (Variables|Default|GetSpline)) (Variables|Default|GetMeshLength)) 1.0)))
    (bind _returnvalue (AddComponent|AddSplineMeshComponent false))
    (SplineMesh|SetStartandEnd _returnvalue (Spline|GetLocationatDistanceAlongSpline _spline_2 (* _index (Variables|Default|GetMeshLength)) "Local") (Math|Vector|ClampVectorSize (Spline|GetTangentatDistanceAlongSpline _spline_2 (* _index (Variables|Default|GetMeshLength)) "Local") 0.0 (Variables|Default|GetMeshLength)) (Spline|GetLocationatDistanceAlongSpline _spline (* (+ _index 1) (Variables|Default|GetMeshLength)) "Local") (Math|Vector|ClampVectorSize (Spline|GetTangentatDistanceAlongSpline _spline (* (+ _index 1) (Variables|Default|GetMeshLength)) "Local") 0.0 (Variables|Default|GetMeshLength)) true :!class /Script/Engine.SplineMeshComponent)))